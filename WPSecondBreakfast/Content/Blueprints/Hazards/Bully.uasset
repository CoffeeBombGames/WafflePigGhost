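; Bully is a hazard actor that chases the player within its sight range and returns to its construction-time location otherwise.
; Overlap events set the in-range flag, clearing it after a two-second delay on exit.
; Each tick, a visibility trace picks hunting the player or seeking the last seen position.
; Movement applies an unswept local offset along the target direction, without delta-time scaling, and draws debug traces.
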(event `self.ReceiveTick`
  (params (DeltaSeconds :type "Float (single-precision)"))
  ;[1 1 1] Action Tree
  (set `self.deltaTime` DeltaSeconds)
  (if (`self.TargetInRange`)
    (bind _sightcheck (`self.CheckSight`))
    (if _sightcheck
      (`self.Hunt`)
      (else
        (`self.Seek`)))
    (else
      (`self.return home`)))
  (`self.MoveTo` (`self.MovementTargetLocation`)))

(event `self.SightRange.OnComponentBeginOverlap`
  (params (OtherActor :type "Actor Object Reference") (OtherComp :type "PrimitiveComponent Object Reference") (OtherBodyIndex :type Integer) (bFromSweep :type Boolean) (SweepResult :type "EngineTypes.HitResult Structure (by ref)"))
  (bind _returnvalue (== OtherActor (`GameplayStatics.GetPlayerPawn` 0)))
  ;[1 1 1] Target Sighting
  (if _returnvalue
    (set `self.TargetInRange` _returnvalue)))

(event `self.SightRange.OnComponentEndOverlap`
  (params (OtherActor :type "Actor Object Reference") (OtherComp :type "PrimitiveComponent Object Reference") (OtherBodyIndex :type Integer))
  (bind _returnvalue (== OtherActor (`GameplayStatics.GetPlayerPawn` 0)))
  ;[1 1 1] Target Dropped
  (if _returnvalue
    (`KismetSystemLibrary.Delay` 2.0)
    (set `self.TargetInRange` (not _returnvalue))))

(fn `CheckSight`
  (returns (SightCheck :type Boolean))
  (bind _returnvalue (`self.K2_GetActorLocation` (`GameplayStatics.GetPlayerPawn` 0)))
  ;[1 1 1] Direct sight check
  (bind (_outhit _returnvalue_2) (`KismetSystemLibrary.LineTraceSingle` :`Start` (`self.K2_GetActorLocation`) :`End` _returnvalue :`TraceChannel` "TraceTypeQuery1" :`DrawDebugType` "ForOneFrame"))
  (bind _returnvalue_3 (not _returnvalue_2))
  ;[1 1 1] Save last known if sight broken
  (if _returnvalue_3
    (set `self.targetLastLocation` _returnvalue))
  (return _returnvalue_3))

(fn `Hunt`
  ;[1 1 1] Move towards sighted target
  (set `self.MovementTargetLocation` (`self.K2_GetActorLocation` (`GameplayStatics.GetPlayerPawn` 0))))

(fn `MoveTo`
  (params (Location :type "Object.Vector Structure"))
  (bind _returnvalue (`self.K2_GetActorLocation`))
  (`self.K2_AddActorLocalOffset` (`KismetMathLibrary.GetDirectionVector` _returnvalue Location))
  (`KismetSystemLibrary.LineTraceSingle` :`Start` _returnvalue :`End` Location :`TraceChannel` "TraceTypeQuery1" :`DrawDebugType` "ForOneFrame"))

(fn `return home`
  (set `self.MovementTargetLocation` (`self.home`)))

(fn `Seek`
  (set `self.MovementTargetLocation` (`self.targetLastLocation`)))

(fn `UserConstructionScript`
  (set `self.home` (`self.K2_GetActorLocation`)))