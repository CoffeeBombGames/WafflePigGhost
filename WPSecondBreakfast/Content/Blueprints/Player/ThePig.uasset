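; ThePig is the player pawn, moved by UpDown and LeftRight axis inputs along its forward and right vectors.
; The construction script stores its starting location as Home, which UpdateHome can replace with a new respawn point.
; Death teleports the pig back to Home without sweeping, while the Damage function is an empty stub.
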(event `InputAxis|UpDown`
  (params (AxisValue :type "Float (single-precision)"))
  (`self.AddMovementInput` (`self.GetActorForwardVector`) AxisValue))

(event `InputAxis|LeftRight`
  (params (AxisValue :type "Float (single-precision)"))
  (`self.AddMovementInput` (`self.GetActorRightVector`) AxisValue))

(fn `Damage`)

(fn `Death`
  (`self.K2_SetActorLocation` (`self.Home`)))

(fn `UpdateHome`
  (params (NewHome :type "Object.Vector Structure"))
  (set `self.Home` NewHome))

(fn `UserConstructionScript`
  (set `self.Home` (`self.K2_GetActorLocation`)))