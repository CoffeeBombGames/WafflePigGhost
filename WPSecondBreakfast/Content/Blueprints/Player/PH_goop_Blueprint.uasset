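; Short-lived goop actor in the Player folder, tagged "Syrup" so it can be identified by that tag.
; The construction script sets the tag and snaps the actor's height to a fixed offset below the first player pawn, keeping its own X and Y.
; After BeginPlay it waits a few seconds and destroys itself.
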(event `self.ReceiveBeginPlay`
  (`KismetSystemLibrary.Delay` 5.0)
  (`self.K2_DestroyActor`))

(fn `UserConstructionScript`
  (set `self.Tags` (`|MakeArray` "Syrup" :!type "Name"))
  (`self.K2_SetActorLocation` (`KismetMathLibrary.MakeVector` (.x (`self.K2_GetActorLocation`)) (.y (`self.K2_GetActorLocation`)) (+ (.z (`self.K2_GetActorLocation` (`GameplayStatics.GetPlayerPawn` 0))) -50.0))))