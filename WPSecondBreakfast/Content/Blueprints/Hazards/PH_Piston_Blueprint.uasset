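; Piston hazard that shuttles between Start and End points and kills the player's pig on contact.
; Each tick, UpdateLerpValue ping-pongs CurrentState by delta time between zero and Switchoffvalue, and Movement uses it directly as the lerp alpha to set the actor location without sweeping.
; A RootBox begin overlap with player pawn 0 casts it to ThePig and calls Death.
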(event `self.ReceiveTick`
  (params (DeltaSeconds :type "Float (single-precision)"))
  (set `self.DeltaTime` DeltaSeconds)
  (`self.UpdateLerpValue`)
  (`self.Movement`))

(event `self.rootBox.OnComponentBeginOverlap`
  (params (OtherActor :type "Actor Object Reference") (OtherComp :type "PrimitiveComponent Object Reference") (OtherBodyIndex :type Integer) (bFromSweep :type Boolean) (SweepResult :type "EngineTypes.HitResult Structure (by ref)"))
  ;[1 1 1] Damage the piggy
  (if (== OtherActor (`GameplayStatics.GetPlayerPawn` 0))
    (bind _asthe_pig (cast `/Game/Blueprints/Player/ThePig` OtherActor))
    (`/Game/Blueprints/Player/ThePig.Death` _asthe_pig)))

(fn `Movement`
  (`self.K2_SetActorLocation` (`KismetMathLibrary.VLerp` (`self.Start`) (`self.End`) (`self.currentState`)))
  (return))

(fn `UpdateLerpValue`
  (bind _currentstate (`self.currentState`))
  (bind _currentstate_2 (`self.currentState`))
  (if (`self.switch`)
    (set `self.currentState` (+ _currentstate (`self.DeltaTime`)))
    (if (> _currentstate (`self.switchoffvalue`))
      (set `self.switch` false))
    (else
      (set `self.currentState` (- _currentstate_2 (`self.DeltaTime`)))
      (if (> 0.0 _currentstate_2)
        (set `self.switch` true))))
  (return))

(fn `UserConstructionScript`)