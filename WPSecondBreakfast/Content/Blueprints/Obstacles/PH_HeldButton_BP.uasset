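; PH_HeldButton_BP is an obstacle button that the player can hold down with goo.
; Overlapping the capsule enables input, so pressing btn1 or btn4 shows the Goo component, sets HeldDown and disables input.
; Leaving the capsule while HeldDown is false disables input, sets the button's relative location and calls Reverse on Target.
; Once HeldDown is set, nothing here clears it, so leaving no longer reverses Target.
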(event `InputAction|btn1`
  (:`Pressed`
    (`SceneComponent.SetVisibility` (`self.goo`) true false :!label _label)
    (set `self.HeldDown` true)
    (`self.DisableInput` (`GameplayStatics.GetPlayerController` 0))))

(event `self.Capsule1.OnComponentBeginOverlap`
  (params (OtherActor :type "Actor Object Reference") (OtherComp :type "PrimitiveComponent Object Reference") (OtherBodyIndex :type Integer) (bFromSweep :type Boolean) (SweepResult :type "EngineTypes.HitResult Structure (by ref)"))
  (if (== OtherActor (`GameplayStatics.GetPlayerPawn` 0))
    (`self.EnableInput` (`GameplayStatics.GetPlayerController` 0))))

(event `InputAction|btn4`
  (:`Pressed`
    (goto _label)))

(event `self.Capsule1.OnComponentEndOverlap`
  (params (OtherActor :type "Actor Object Reference") (OtherComp :type "PrimitiveComponent Object Reference") (OtherBodyIndex :type Integer))
  (if (== OtherActor (`GameplayStatics.GetPlayerPawn` 0))
    (if (not (`self.HeldDown`))
      (`self.DisableInput` (`GameplayStatics.GetPlayerController` 0))
      (`SceneComponent.K2_SetRelativeLocation` (`self.PH_Button_0`) (0.0 0.0 -20.0) false)
      (`MatineeActor.Reverse` (`self.target`)))))

(fn `UserConstructionScript`
  (`parent.UserConstructionScript`))