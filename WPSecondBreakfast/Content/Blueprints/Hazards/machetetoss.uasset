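; Falling machete hazard that kills the player's pig on contact.
; Each tick it moves straight down by DropSpeed scaled by delta time, without sweeping, and destroys itself once it drops below a fixed height.
; Overlapping the first player's pawn casts it to ThePig and calls its Death function.
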(event `self.ReceiveTick`
  (params (DeltaSeconds :type "Float (single-precision)"))
  (bind _returnvalue (- (`self.K2_GetActorLocation`) (`KismetMathLibrary.MakeVector` 0.0 0.0 (* (`self.dropSpeed`) (`self.deltaTime`)))))
  (set `self.deltaTime` DeltaSeconds)
  (`self.K2_SetActorLocation` _returnvalue)
  (if (< (.z _returnvalue) -100.0)
    (`self.K2_DestroyActor`)))

(event `self.ReceiveActorBeginOverlap`
  (params (OtherActor :type "Actor Object Reference"))
  (if (== OtherActor (`GameplayStatics.GetPlayerPawn` 0))
    (bind _asthe_pig (cast `/Game/Blueprints/Player/ThePig` OtherActor))
    (`/Game/Blueprints/Player/ThePig.Death` _asthe_pig)))

(fn `UserConstructionScript`)